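; Game mode for a game with procedurally chained road pieces that also manages the start, in-game and end menus.
; On BeginPlay it plays background music, spawns an initial run of roads and shows the start menu with character input disabled.
; AddRoad places each Road at the previous piece's attach transform.
; ClickedPlay restores input and shows the HUD, while EndMenu disables input and shows the end screen.
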(event `EndMenu`
  (bind _returnvalue (`GameplayStatics.GetPlayerController` 0))
  (`self.DisableInput` _returnvalue)
  (bind _returnvalue_2 (`|CreateWidget` "/Game/Blueprints/EndMenu.EndMenu_C"))
  (`UserWidget.AddToViewport` _returnvalue_2 0)
  (bind _output_get (set `PlayerController.bEnableMouseOverEvents` true _returnvalue))
  (set `PlayerController.bShowMouseCursor` _output_get _returnvalue)
  (`WidgetBlueprintLibrary.SetInputMode_UIOnlyEx` null _returnvalue_2))

(event `self.ReceiveBeginPlay`
  (bind _returnvalue (`GameplayStatics.GetPlayerController` 0))
  ;[1 1 1] Generates 6 new road pieces
  (`|ExecutionSequence`
    (:`then_0`
      (`GameplayStatics.PlaySound2D` "/Game/Audio/Starter_Background_Cue.Starter_Background_Cue"))
    (:`then_1`
      (for _ (range 6)
        (`self.AddRoad`)))
    (:`then_2`
      ;[1 1 1] Start menu
      (`self.DisableInput` (`GameplayStatics.GetPlayerCharacter` 0) null)
      (bind _returnvalue_2 (`|CreateWidget` "/Game/Blueprints/StartMenu.StartMenu_C"))
      (`UserWidget.AddToViewport` _returnvalue_2 0)
      (bind _output_get (set `PlayerController.bEnableMouseOverEvents` true _returnvalue))
      (set `PlayerController.bShowMouseCursor` _output_get _returnvalue)
      (`WidgetBlueprintLibrary.SetInputMode_UIOnlyEx` _returnvalue _returnvalue_2))))

(event `ClickedPlay`
  (bind _returnvalue (`GameplayStatics.GetPlayerController` 0))
  ;[1 1 1] Clicked play button removes startmenu and activates ingame menu
  (`self.EnableInput` (`GameplayStatics.GetPlayerCharacter` 0) null)
  (bind _output_get (set `PlayerController.bEnableMouseOverEvents` false _returnvalue))
  (set `PlayerController.bShowMouseCursor` _output_get _returnvalue)
  (bind _returnvalue_2 (`|CreateWidget` "/Game/Blueprints/InGameHUD.InGameHUD_C"))
  (`UserWidget.AddToViewport` _returnvalue_2 0))

(fn `AddRoad`
  ;[1 1 1] Spawns new road
  (bind _returnvalue (`|SpawnActorFromClass` "/Game/Blueprints/Road.Road_C" (`self.NextSpawnPoint`) "Undefined" "OverrideRootScale"))
  (bind _attachtransform (`/Game/Blueprints/Road.GetAttachTransform` _returnvalue))
  (set `self.NextSpawnPoint` _attachtransform))

(fn `UserConstructionScript`)