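; LTruck is a truck obstacle that drives along world Y and hurts the player on contact.
; Each Tick it re-caches the player's MyCharacter, moves at that character's CarSpeed scaled by delta time, and creates and assigns a new dynamic material instance on CarMesh.
; On overlap with a MyCharacter, if the cached capsule is tagged Player, it calls VehicleHit, briefly flashes HurtScreen, then destroys itself.
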(event `self.ReceiveTick`
  (params (DeltaSeconds :type "Float (single-precision)"))
  ;[1 1 1] Car movement
  ;[1 1 1] MyCharacter reference
  (`|ExecutionSequence`
    (:`then_0`
      (bind _asmy_character (cast `/Game/Blueprints/MyCharacter` (`GameplayStatics.GetPlayerCharacter` 0)))
      (set `self.CharacterReference` _asmy_character))
    (:`then_1`
      (`self.K2_AddActorWorldOffset` (`KismetMathLibrary.MakeVector` 0.0 (* DeltaSeconds (`/Game/Blueprints/MyCharacter.CarSpeed` (`self.CharacterReference`))))))
    (:`then_2`
      (bind _returnvalue (`PrimitiveComponent.CreateDynamicMaterialInstance` (`self.CarMesh`) 0 "/Game/Materials/MAT_CarMaterial.MAT_CarMaterial"))
      (`PrimitiveComponent.SetMaterial` (`self.CarMesh`) 0 _returnvalue))))

(event `self.CarMesh.OnComponentBeginOverlap`
  (params (OtherActor :type "Actor Object Reference") (OtherComp :type "PrimitiveComponent Object Reference") (OtherBodyIndex :type Integer) (bFromSweep :type Boolean) (SweepResult :type "HitResult Structure (by ref)"))
  (bind _hurtscreen (`/Game/Blueprints/MyCharacter.HurtScreen` (`self.CharacterReference`)))
  ;[1 1 1] Calls hurt event in MyCharacter blueprint
  (bind _asmy_character (cast `/Game/Blueprints/MyCharacter` OtherActor))
  (if (`ActorComponent.ComponentHasTag` (`Character.CapsuleComponent` (`self.CharacterReference`)) "Player")
    (set `PostProcessComponent.bEnabled` true _hurtscreen)
    (`/Game/Blueprints/MyCharacter.VehicleHit` _asmy_character)
    (`KismetSystemLibrary.Delay` 0.2)
    (set `PostProcessComponent.bEnabled` false _hurtscreen)
    (`self.K2_DestroyActor`)))

(fn `UserConstructionScript`)