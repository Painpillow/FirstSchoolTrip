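; RVehicle is a vehicle hazard that drives along the world Y axis and hurts the player character on contact.
; Each Tick it re-casts and stores the player as MyCharacter, then offsets itself by a frame-time-scaled value derived from that character's CarSpeed.
; When a MyCharacter overlaps its HurtTrigger, it calls VehicleHit, the character's death event, and destroys itself.
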(event `self.ReceiveTick`
  (params (DeltaSeconds :type "Float (single-precision)"))
  ;[1 1 1] Car movement
  ;[1 1 1] MyCharacter reference
  (`|ExecutionSequence`
    (:`then_0`
      (bind _asmy_character (cast `/Game/Blueprints/MyCharacter` (`GameplayStatics.GetPlayerCharacter` 0)))
      (set `self.CharacterReference` _asmy_character))
    (:`then_1`
      (bind _result (`/Engine/EditorBlueprintResources/StandardMacros.NegateFloat` (* DeltaSeconds (`/Game/Blueprints/MyCharacter.CarSpeed` (`self.CharacterReference`))))
        (:`  `
          (`self.K2_AddActorWorldOffset` (`KismetMathLibrary.MakeVector` 0.0 _result)))))))

(event `self.HurtTrigger.OnComponentBeginOverlap`
  (params (OtherActor :type "Actor Object Reference") (OtherComp :type "PrimitiveComponent Object Reference") (OtherBodyIndex :type Integer) (bFromSweep :type Boolean) (SweepResult :type "HitResult Structure (by ref)"))
  ;[1 1 1] Calls death event in MyCharacter blueprint
  (bind _asmy_character (cast `/Game/Blueprints/MyCharacter` OtherActor))
  (`/Game/Blueprints/MyCharacter.VehicleHit` _asmy_character)
  (`self.K2_DestroyActor`))

(fn `UserConstructionScript`)