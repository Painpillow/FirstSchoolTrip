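; Road segment actor for an endless road-crossing game, which scores the player's crossing and spawns traffic on both sides.
; Its score trigger updates the character's crossing count and vehicle speed, then removes itself, while a destroy trigger asks the game mode for a new road and self-destructs after a delay.
; A Delay on Tick, randomized up to the character's spawn rate, paces child-actor car spawns, and side triggers destroy matching vehicles.
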(event `self.ScoreTrigger.OnComponentBeginOverlap`
  (params (OtherActor :type "Actor Object Reference") (OtherComp :type "PrimitiveComponent Object Reference") (OtherBodyIndex :type Integer) (bFromSweep :type Boolean) (SweepResult :type "HitResult Structure (by ref)"))
  ;[1 1 1] +1 Road crossed
  (bind _asmy_character (cast `/Game/Blueprints/MyCharacter` OtherActor))
  (`/Game/Blueprints/MyCharacter.RoadCrossed` _asmy_character)
  (`/Game/Blueprints/MyCharacter.VehicleSpeed` _asmy_character))

(event `self.DestroyTrigger.OnComponentBeginOverlap`
  (params (OtherActor :type "Actor Object Reference") (OtherComp :type "PrimitiveComponent Object Reference") (OtherBodyIndex :type Integer) (bFromSweep :type Boolean) (SweepResult :type "HitResult Structure (by ref)"))
  ;[1 1 1] Generate and destroy road
  (cast `/Game/Blueprints/MyCharacter` OtherActor)
  (bind _ascustom_game_mode (cast `/Game/Blueprints/CustomGameMode` (`GameplayStatics.GetGameMode`)))
  (`/Game/Blueprints/CustomGameMode.AddRoad` _ascustom_game_mode)
  (`KismetSystemLibrary.Delay` 1.0)
  (`self.K2_DestroyActor`))

(event `self.R_CarDestroyTrigger.OnComponentBeginOverlap`
  (params (OtherActor :type "Actor Object Reference") (OtherComp :type "PrimitiveComponent Object Reference") (OtherBodyIndex :type Integer) (bFromSweep :type Boolean) (SweepResult :type "HitResult Structure (by ref)"))
  ;[1 1 1] Destroys cars
  (bind _asrvehicle (cast `/Game/Blueprints/RVehicle` OtherActor))
  (`self.K2_DestroyActor` _asrvehicle))

(event `self.ReceiveBeginPlay`
  ;[1 1 1] MyCharacter reference
  (bind _asmy_character (cast `/Game/Blueprints/MyCharacter` (`GameplayStatics.GetPlayerCharacter` 0)))
  (set `self.CharacterReference` _asmy_character))

(event `self.L_CarDestroyTrigger.OnComponentBeginOverlap`
  (params (OtherActor :type "Actor Object Reference") (OtherComp :type "PrimitiveComponent Object Reference") (OtherBodyIndex :type Integer) (bFromSweep :type Boolean) (SweepResult :type "HitResult Structure (by ref)"))
  ;[1 1 1] Destroys cars
  (bind _aslvehicle (cast `/Game/Blueprints/LVehicle` OtherActor))
  (`self.K2_DestroyActor` _aslvehicle))

(event `self.ScoreTrigger.OnComponentEndOverlap`
  (params (OtherActor :type "Actor Object Reference") (OtherComp :type "PrimitiveComponent Object Reference") (OtherBodyIndex :type Integer))
  ;[1 1 1] Destroy score trigger
  (`ActorComponent.K2_DestroyComponent` (`self.ScoreTrigger`)))

(event `self.ReceiveTick`
  (params (DeltaSeconds :type "Float (single-precision)"))
  ;[1 1 1] Spawns cars
  (`KismetSystemLibrary.Delay` (`KismetMathLibrary.RandomFloatInRange` 1.0 (`/Game/Blueprints/MyCharacter.CarSpawnRate` (`self.CharacterReference`))))
  (`/Engine/EditorBlueprintResources/StandardMacros.CompareFloat` (`KismetMathLibrary.RandomFloat`) 0.3
    (:`>`
      (`AddComponent|ChildActorComponent_4` :`RelativeTransform` (`SceneComponent.GetRelativeTransform` (`self.R_CarSpawn`))))
    (:`==`
      (`AddComponent|Child Actor Component_2` :`RelativeTransform` (`SceneComponent.GetRelativeTransform` (`self.R_CarSpawn`)) :!label _label))
    (:`<`
      (goto _label)))
  (`/Engine/EditorBlueprintResources/StandardMacros.CompareFloat` (`KismetMathLibrary.RandomFloat`) 0.3
    (:`>`
      (`AddComponent|ChildActorComponent_5` :`RelativeTransform` (`SceneComponent.GetRelativeTransform` (`self.L_CarSpawn`))))
    (:`==`
      (`AddComponent|Child Actor Component_16` :`RelativeTransform` (`SceneComponent.GetRelativeTransform` (`self.L_CarSpawn`)) :!label _label_2))
    (:`<`
      (goto _label_2))))

(fn `GetAttachTransform`
  (returns (AttachTransform :type "Transform Structure"))
  ;[1 1 1] Road attach point
  (return (`SceneComponent.K2_GetComponentToWorld` (`self.AttachPoint`))))

(fn `UserConstructionScript`)